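; BP_ActorVideoEncoder is a scene-capture actor, named for video encoding, that sweeps a downward-tilted view around while showing a capture widget on screen.
; It assigns its SceneCapture component to the SceneCaptureComponent2D variable in both the construction script and BeginPlay.
; BeginPlay also adds WBP_SceneCapture to the viewport.
; Tick holds a fixed pitch and advances yaw by delta time for a steady, frame-rate-independent spin.
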(event `self.ReceiveBeginPlay`
  (set `self.SceneCaptureComponent2D` (`self.SceneCapture`))
  (bind _returnvalue (`|CreateWidget` "/Game/WBP_SceneCapture.WBP_SceneCapture_C"))
  (`UserWidget.AddToViewport` _returnvalue 0))

(event `self.ReceiveTick`
  (params (DeltaSeconds :type "Float (single-precision)"))
  (bind (_returnvalue_roll _returnvalue_pitch _returnvalue_yaw) (`KismetMathLibrary.BreakRotator` (`self.K2_GetActorRotation`)))
  (`self.K2_SetActorRotation` (`KismetMathLibrary.MakeRotator` 0.0 -50.0 (+ (* DeltaSeconds 10.0) _returnvalue_yaw))))

(fn `UserConstructionScript`
  (set `self.SceneCaptureComponent2D` (`self.SceneCapture`)))